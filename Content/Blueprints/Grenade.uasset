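; Grenade actor that bursts into a magic-sphere particle effect on impact and destroys itself, with no damage logic.
; A capsule hit on any other actor prints a debug string, calls the ExplosionParticle event in a short loop, then destroys the grenade.
; ExplosionParticle spawns the half-scale emitter at the grenade's location behind an authority check, so it runs only on the authority side.
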(event `ExplosionParticle`
  (`/Engine/EditorBlueprintResources/ActorMacros.Switch Has Authority`
    (:`Authority`
      (`GameplayStatics.SpawnEmitterAtLocation` "/Game/RPGEffects/Particles/P_Mage_MagicSphere.P_Mage_MagicSphere" (`self.K2_GetActorLocation`) (struct) (0.5 0.5 0.5)))))

(event `self.Capsule.OnComponentHit`
  (params (HitComponent :type "PrimitiveComponent Object Reference") (OtherActor :type "Actor Object Reference") (OtherComp :type "PrimitiveComponent Object Reference") (NormalImpulse :type "Vector Structure") (Hit :type "HitResult Structure (by ref)"))
  (`KismetSystemLibrary.PrintString` "Hello")
  (if (!= OtherActor self)
    (for _ (range 2)
      (`self.ExplosionParticle`))
    (`self.K2_DestroyActor`)))

(fn `UserConstructionScript`)